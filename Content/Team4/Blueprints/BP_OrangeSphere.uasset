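; BP_OrangeSphere is an interactable sphere actor that shows a billboard indicator when the player is nearby.
; On BeginPlay it caches the player as a BP_ThirdPersonCharacter, and overlaps on Sphere1 toggle the billboard's visibility for that player only.
; Its Interact event currently just prints a debug message.
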(event `self.ReceiveBeginPlay`
  (bind _asbp_third_person_character (cast `/Game/ThirdPerson/Blueprints/BP_ThirdPersonCharacter` (`GameplayStatics.GetPlayerCharacter` 0)))
  (set `self.PlayerRef` _asbp_third_person_character))

(event `/Game/Team4/Blueprints/Interfaces/BPI_Interact.Interact`
  (`KismetSystemLibrary.PrintString` "Interacted with Orange Sphere"))

(event `self.Sphere1.OnComponentBeginOverlap`
  (params (OverlappedComponent :type "PrimitiveComponent Object Reference") (OtherActor :type "Actor Object Reference") (OtherComp :type "PrimitiveComponent Object Reference") (OtherBodyIndex :type Integer) (bFromSweep :type Boolean) (SweepResult :type "HitResult Structure (by ref)"))
  (if (== OtherActor (`self.PlayerRef`))
    (`SceneComponent.SetVisibility` (`self.Billboard`) true false)))

(event `self.Sphere1.OnComponentEndOverlap`
  (params (OverlappedComponent :type "PrimitiveComponent Object Reference") (OtherActor :type "Actor Object Reference") (OtherComp :type "PrimitiveComponent Object Reference") (OtherBodyIndex :type Integer))
  (if (== (`self.PlayerRef`) OtherActor)
    (`SceneComponent.SetVisibility` (`self.Billboard`) false false)))

(fn `UserConstructionScript`)